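; Lighting preset actor that sets a level's time of day: Overcast, Midday, Sunset, Dusk/Dawn or Night.
; The Construction Script switches on TimeOfDay to show that preset's directional light, fog and skylight, recapture the sky and enable dynamic indirect lighting.
; SunAngleZ sets the active light's yaw while preserving pitch and roll.
; Only Overcast hides anything (AtmosphericFog), and nothing runs at runtime.
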(fn `UserConstructionScript`
  (bind _midday_directional (`self.Midday_Directional`))
  (bind _midday_skylight (`self.Midday_Skylight`))
  (bind _sunset_skylight (`self.Sunset_Skylight`))
  (bind _sunset_directional (`self.Sunset_Directional`))
  (bind _dusk_directional (`self.Dusk_Directional`))
  (bind _dusk_skylight (`self.Dusk_Skylight`))
  (bind _overcast_directional (`self.Overcast_Directional`))
  (bind _overcast_skylight (`self.Overcast_Skylight`))
  (bind _night_skylight (`self.Night_Skylight`))
  (bind _night_directional (`self.Night_Directional`))
  (switch `/Game/Environments/Reference/BP/TimeOfDay_list` (`self.Time of Day`)
    (:`NewEnumerator0`
      ;[1 1 1] Overcast
      (`LightComponent.SetAffectDynamicIndirectLighting` _overcast_directional true)
      (`SceneComponent.K2_SetWorldRotation` _overcast_directional (`KismetMathLibrary.MakeRotator` (.roll (`SceneComponent.K2_GetComponentRotation` _overcast_directional)) (.pitch (`SceneComponent.K2_GetComponentRotation` _overcast_directional)) (`KismetMathLibrary.Conv_IntToDouble` (`self.Sun Angle (Z)`))) false false)
      (`SceneComponent.SetVisibility` _overcast_directional true false)
      (`SceneComponent.SetVisibility` (`self.Overcast_Fog`) true false)
      (`SkyLightComponent.RecaptureSky` _overcast_skylight)
      (`SceneComponent.SetVisibility` _overcast_skylight true false)
      (`SceneComponent.SetVisibility` (`self.AtmosphericFog`) false false))
    (:`NewEnumerator1`
      ;[1 1 1] Midday
      (`LightComponent.SetAffectDynamicIndirectLighting` _midday_directional true)
      (`SceneComponent.K2_SetWorldRotation` _midday_directional (`KismetMathLibrary.MakeRotator` (.roll (`SceneComponent.K2_GetComponentRotation` _midday_directional)) (.pitch (`SceneComponent.K2_GetComponentRotation` _midday_directional)) (`KismetMathLibrary.Conv_IntToDouble` (`self.Sun Angle (Z)`))) false false)
      (`SceneComponent.SetVisibility` _midday_directional true false)
      (`SceneComponent.SetVisibility` (`self.Midday_Fog`) true false)
      (`SkyLightComponent.RecaptureSky` _midday_skylight)
      (`SceneComponent.SetVisibility` _midday_skylight true false))
    (:`NewEnumerator2`
      ;[1 1 1] Sunset
      (`LightComponent.SetAffectDynamicIndirectLighting` _sunset_directional true)
      (`SceneComponent.K2_SetWorldRotation` _sunset_directional (`KismetMathLibrary.MakeRotator` (.roll (`SceneComponent.K2_GetComponentRotation` _sunset_directional)) (.pitch (`SceneComponent.K2_GetComponentRotation` _sunset_directional)) (`KismetMathLibrary.Conv_IntToDouble` (`self.Sun Angle (Z)`))) false false)
      (`SceneComponent.SetVisibility` _sunset_directional true false)
      (`SceneComponent.SetVisibility` (`self.Sunset_Fog`) true false)
      (`SkyLightComponent.RecaptureSky` _sunset_skylight)
      (`SceneComponent.SetVisibility` _sunset_skylight true false))
    (:`NewEnumerator3`
      ;[1 1 1] Dusk/Dawn
      (`LightComponent.SetAffectDynamicIndirectLighting` _dusk_directional true)
      (`SceneComponent.K2_SetWorldRotation` _dusk_directional (`KismetMathLibrary.MakeRotator` (.roll (`SceneComponent.K2_GetComponentRotation` _dusk_directional)) (.pitch (`SceneComponent.K2_GetComponentRotation` _dusk_directional)) (`KismetMathLibrary.Conv_IntToDouble` (`self.Sun Angle (Z)`))) false false)
      (`SceneComponent.SetVisibility` _dusk_directional true false)
      (`SceneComponent.SetVisibility` (`self.Dusk_Fog`) true false)
      (`SkyLightComponent.RecaptureSky` _dusk_skylight)
      (`SceneComponent.SetVisibility` _dusk_skylight true false))
    (:`NewEnumerator4`
      ;[1 1 1] Night
      (`LightComponent.SetAffectDynamicIndirectLighting` _night_directional true)
      (`SceneComponent.K2_SetWorldRotation` _night_directional (`KismetMathLibrary.MakeRotator` (.roll (`SceneComponent.K2_GetComponentRotation` _night_directional)) (.pitch (`SceneComponent.K2_GetComponentRotation` _night_directional)) (`KismetMathLibrary.Conv_IntToDouble` (`self.Sun Angle (Z)`))) false false)
      (`SceneComponent.SetVisibility` _night_skylight true false)
      (`SceneComponent.SetVisibility` _night_directional true false)
      (`SceneComponent.SetVisibility` (`self.Night_Fog`) true false)
      (`SkyLightComponent.RecaptureSky` _night_skylight)
      (`SceneComponent.SetVisibility` _night_skylight true false))))